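; Player car Blueprint that handles driving, air control, enemy scanning, damage from Enemy- or Civilian-tagged actors and HUD creation.
; A downward trace each Tick gates throttle and steering, switching them to mesh torque when airborne and driving velocity-based particle trails when grounded.
; Tick also counters roll and rights flipped cars.
; Scan inputs query Level_Manager or sphere-trace for WeakPointInterface actors to display weakspots; others handle handbrake, reverse, respawn and restart.
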(event `InputAction|Reset Position`
  (params (Key :type "Key Structure"))
  ;[1 1 1] Respawn at player start
  (:`Pressed`
    (bind _returnvalue (`GameplayStatics.GetActorOfClass` "/Script/Engine.PlayerStart"))
    (`self.K2_TeleportTo` :`self` (`GameplayStatics.GetPlayerPawn` 0) :`DestLocation` (`self.K2_GetActorLocation` _returnvalue))))

(event `InputAction|Quit Level`
  (params (Key :type "Key Structure"))
  ;[1 1 1] Quit level TODO: spawn back in level select
  (:`Pressed`
    (bind _asgame_mode (cast `GameMode` (`GameplayStatics.GetGameMode`))
      (:`then`
        (`GameMode.RestartGame` _asgame_mode))
      (:`CastFailed`
        (`KismetSystemLibrary.PrintString` "cast to gamemode failed")))))

(event `self.ReceiveTick`
  (params (DeltaSeconds :type "Float (single-precision)"))
  (bind (_returnvalue_x _returnvalue_y _returnvalue_z) (`KismetMathLibrary.BreakVector` (`self.GetActorUpVector`)))
  (bind (_returnvalue_roll _returnvalue_pitch _returnvalue_yaw) (`KismetMathLibrary.BreakRotator` (`self.K2_GetActorRotation`)))
  (bind _mesh (`self.Mesh`))
  (bind _returnvalue (`SceneComponent.GetForwardVector` _mesh))
  (bind _roll (.roll (`self.K2_GetActorRotation`)))
  (bind _returnvalue_2 (`SceneComponent.K2_GetComponentLocation` (`MovementComponent.UpdatedPrimitive` (`self.VehicleMovementComponent`))))
  ;[1 1 1] reset vehicle if flipped
  (if (< _returnvalue_z 0.0)
    (`KismetSystemLibrary.Delay` 2.0)
    (`self.K2_TeleportTo` (+ (`self.K2_GetActorLocation`) (0.0 0.0 200.0)) (`KismetMathLibrary.MakeRotator` 0.0 0.0 _returnvalue_yaw)))
  ;[1 1 1] Input mapping and smoke trails
  (bind (_outhit _returnvalue_3) (`KismetSystemLibrary.LineTraceSingle` _returnvalue_2 (+ _returnvalue_2 (0.0 0.0 -100.0)) "TraceTypeQuery1"))
  (if (and (>= _roll 90.0) (<= _roll 180.0))
    (`PrimitiveComponent.AddTorqueInDegrees` _mesh (* _returnvalue -1000000000.0) "None" false)
    (elif (and (<= _roll 270.0) (>= _roll 180.0))
      (`PrimitiveComponent.AddTorqueInDegrees` _mesh (* _returnvalue 1000000000.0) "None" false))))

(event `InputAxis|Throttle`
  (params (AxisValue :type "Float (single-precision)"))
  (bind _returnvalue (`self.GetVelocity`))
  (bind _vehiclemovementcomponent (`self.VehicleMovementComponent`))
  (bind _mesh (`self.Mesh`))
  (bind _particle_test (`self.particle_test`))
  (bind _returnvalue_2 (`KismetMathLibrary.Dot_VectorVector` (`self.GetActorForwardVector`) _returnvalue))
  (bind _returnvalue_3 (`KismetMathLibrary.VSize` _returnvalue))
  ;[1 1 1] Input mapping and smoke trails
  (if (stale `self.ReceiveTick` _returnvalue_3)
    (`ChaosVehicleMovementComponent.SetThrottleInput` _vehiclemovementcomponent AxisValue)
    (`FXSystemComponent.SetEmitterEnable` _particle_test "ConfettiBurst" (and (<= _returnvalue_2 (+ (/ _returnvalue_3 1.0) -100.0)) (> _returnvalue_3 200.0)))
    (`FXSystemComponent.SetFloatParameter` _particle_test "rate" (/ 80000.0 (`KismetMathLibrary.Abs` (+ _returnvalue_2 400.0))))
    (else
      (`ChaosVehicleMovementComponent.SetThrottleInput` _vehiclemovementcomponent 0.0)
      (`FXSystemComponent.SetEmitterEnable` (`self.particle_test`) "ConfettiBurst" false)
      (`PrimitiveComponent.AddTorqueInDegrees` _mesh (* (`SceneComponent.GetForwardVector` _mesh) (* (stale `InputAxis|Steering` AxisValue) -500000000.0)) "None" false))))

(event `InputAxis|Steering`
  (params (AxisValue :type "Float (single-precision)"))
  (bind _vehiclemovementcomponent (`self.VehicleMovementComponent`))
  (bind _mesh (`self.Mesh`))
  ;[1 1 1] Input mapping and smoke trails
  (if (stale `self.ReceiveTick` _returnvalue_3)
    (`ChaosVehicleMovementComponent.SetSteeringInput` _vehiclemovementcomponent AxisValue)
    (else
      (`ChaosVehicleMovementComponent.SetSteeringInput` _vehiclemovementcomponent 0.0)
      (`PrimitiveComponent.AddTorqueInDegrees` _mesh (* (`SceneComponent.GetRightVector` _mesh) (* (stale `InputAxis|Throttle` AxisValue) 500000000.0)) "None" false))))

(event `InputAction|Handbrake`
  (params (Key :type "Key Structure"))
  (bind _vehiclemovementcomponent (`self.VehicleMovementComponent`))
  ;[1 1 1] Input mapping and smoke trails
  (:`Pressed`
    (`ChaosVehicleMovementComponent.SetHandbrakeInput` _vehiclemovementcomponent true))
  (:`Released`
    (`ChaosVehicleMovementComponent.SetHandbrakeInput` _vehiclemovementcomponent false)))

(event `InputAction|Reverse`
  (params (Key :type "Key Structure"))
  (bind _vehiclemovementcomponent (`self.VehicleMovementComponent`))
  ;[1 1 1] Input mapping and smoke trails
  (:`Pressed`
    (`ChaosVehicleMovementComponent.SetBrakeInput` _vehiclemovementcomponent 0.0)
    (`ChaosVehicleMovementComponent.SetTargetGear` _vehiclemovementcomponent -1 true)
    (`ChaosVehicleMovementComponent.SetThrottleInput` _vehiclemovementcomponent 1.0))
  (:`Released`
    (`ChaosVehicleMovementComponent.SetTargetGear` _vehiclemovementcomponent 0 true)))

(event `InputAction|ScanForEnemies`
  (params (Key :type "Key Structure"))
  ;[1 1 1] Scan for enemies
  (:`Pressed`
    (bind _returnvalue (`GameplayStatics.GetActorOfClass` "/Game/JJ_level/Level_Manager.Level_Manager_C"))
    (`/Game/JJ_level/Level_Manager.PlayerRequestLocation_Event` _returnvalue)))

(event `InputAction|Find Weakspots`
  (params (Key :type "Key Structure"))
  (bind _returnvalue (`self.K2_GetActorLocation`))
  ;[1 1 1] Scan for and display nearby weakspots
  (:`Pressed`
    (bind _outhits (`KismetSystemLibrary.SphereTraceMultiByProfile` _returnvalue _returnvalue 4000.0 "Pawn"))
    (for _array_element _outhits
      (bind (_bblockinghit _binitialoverlap _time _distance _location _impactpoint _normal _impactnormal _physmat _hitactor) (`GameplayStatics.BreakHitResult` _array_element))
      (if (`KismetSystemLibrary.DoesImplementInterface` _hitactor "/Game/JJ_level/Waves/weakPointInterface.weakPointInterface_C")
        (`KismetSystemLibrary.PrintString` (`KismetSystemLibrary.GetDisplayName` _hitactor))
        (bind _asweak_point_interface (cast `/Game/JJ_level/Waves/weakPointInterface` _hitactor))
        (`/Game/JJ_level/Waves/weakPointInterface.Trigger Weak Point Display` _asweak_point_interface)))))

(event `self.ReceiveAnyDamage`
  (params (Damage :type "Float (single-precision)") (DamageType :type "DamageType Object Reference") (InstigatedBy :type "Controller Object Reference") (DamageCauser :type "Actor Object Reference"))
  ;[1 1 1] Player take damage
  (if (`self.ActorHasTag` DamageCauser "Enemy")
    (set `self.PlayerHealth` (- (`self.PlayerHealth`) Damage) :!label _label)
    (elif (`self.ActorHasTag` DamageCauser "Civilian")
      (goto _label))))

(event `self.ReceiveBeginPlay`
  ;[1 1 1] Player UI
  (bind _returnvalue (`|CreateWidget` "/Game/JJ_level/PlayerUI.PlayerUI_C" (`PlayerState.GetPlayerController` (`GameplayStatics.GetPlayerState` 0))))
  (`UserWidget.AddToViewport` _returnvalue 0))

(fn `UserConstructionScript`)