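; CollectibleBP is a score pickup for the racing level that the player's car collects by driving into it.
; It spins by adding a fixed rotation increment every tick, independent of delta time.
; When its Box overlaps the player pawn, it casts that pawn to CarBP_RACING, adds a base score scaled by the car's Multiplier to its Score, then destroys itself.
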(event `self.ReceiveTick`
  (params (DeltaSeconds :type "Float (single-precision)"))
  (`self.K2_SetActorRotation` (`KismetMathLibrary.ComposeRotators` (`self.K2_GetActorRotation`) (struct :`Yaw` 10.0))))

(event `self.Box.OnComponentBeginOverlap`
  (params (OverlappedComponent :type "PrimitiveComponent Object Reference") (OtherActor :type "Actor Object Reference") (OtherComp :type "PrimitiveComponent Object Reference") (OtherBodyIndex :type Integer) (bFromSweep :type Boolean) (SweepResult :type "HitResult Structure (by ref)"))
  (if (== OtherActor (`GameplayStatics.GetPlayerPawn` 0))
    (bind _ascar_bp_racing (cast `/Game/RacingLevel/CarModel/CarBP_RACING` (`GameplayStatics.GetPlayerPawn` 0)))
    (set `/Game/RacingLevel/CarModel/CarBP_RACING.Score` (+ (`/Game/RacingLevel/CarModel/CarBP_RACING.Score` _ascar_bp_racing) (* (`/Game/RacingLevel/CarModel/CarBP_RACING.Multiplier` _ascar_bp_racing) 500)) _ascar_bp_racing)
    (`self.K2_DestroyActor`)))

(fn `UserConstructionScript`)