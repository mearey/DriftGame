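; BP_GunPowerUp is a shooter pickup that adds a special charge to the player's car.
; When the player pawn overlaps its Sphere, it prints a message and plays a timeline that lerps it from its current location toward the pawn's live position.
; When the timeline finishes, it increments SpecialCharge on CarBP_Shooter, calls FlashBlue and destroys itself.
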(event `self.Sphere.OnComponentBeginOverlap`
  (params (OverlappedComponent :type "PrimitiveComponent Object Reference") (OtherActor :type "Actor Object Reference") (OtherComp :type "PrimitiveComponent Object Reference") (OtherBodyIndex :type Integer) (bFromSweep :type Boolean) (SweepResult :type "HitResult Structure (by ref)"))
  (bind _returnvalue (`GameplayStatics.GetPlayerPawn` 0))
  (if (== OtherActor _returnvalue)
    (`KismetSystemLibrary.PrintString` "Wow you hit a power up potion")
    (bind (_direction _newtrack_0) (`Timeline|Alpha Blend Timeline`)
      (:`Update`
        (`self.K2_SetActorLocation` (`KismetMathLibrary.VLerp` (`self.K2_GetActorLocation`) (`self.K2_GetActorLocation` _returnvalue) _newtrack_0)))
      (:`Finished`
        (bind _ascar_bp_shooter (cast `/Game/shooter_level/CarBP_Shooter` _returnvalue)
          (:`then`
            (set `/Game/shooter_level/CarBP_Shooter.Special Charge` (+ (`/Game/shooter_level/CarBP_Shooter.Special Charge` _ascar_bp_shooter) 1) _ascar_bp_shooter)
            (`/Game/shooter_level/CarBP_Shooter.FlashBlue` _ascar_bp_shooter))
          (:`CastFailed`
            _))
        (`self.K2_DestroyActor`)))))

(fn `UserConstructionScript`)