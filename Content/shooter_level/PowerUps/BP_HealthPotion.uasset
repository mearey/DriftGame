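; Health potion pickup that flies to the player and restores a fixed amount of CarBP health, capped at a maximum.
; When the player pawn overlaps its sphere, it prints a message and plays a timeline that lerps it from its current location toward the pawn's live location.
; When the timeline finishes, it casts the pawn to CarBP, applies the heal and destroys itself.
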(event `self.Sphere.OnComponentBeginOverlap`
  (params (OverlappedComponent :type "PrimitiveComponent Object Reference") (OtherActor :type "Actor Object Reference") (OtherComp :type "PrimitiveComponent Object Reference") (OtherBodyIndex :type Integer) (bFromSweep :type Boolean) (SweepResult :type "HitResult Structure (by ref)"))
  (bind _returnvalue (`GameplayStatics.GetPlayerPawn` 0))
  (if (== OtherActor _returnvalue)
    (`KismetSystemLibrary.PrintString` "Wow you hit a health potion")
    (bind (_direction _newtrack_0) (`Timeline|Alpha Blend Timeline`)
      (:`Update`
        (`self.K2_SetActorLocation` (`KismetMathLibrary.VLerp` (`self.K2_GetActorLocation`) (`self.K2_GetActorLocation` _returnvalue) _newtrack_0)))
      (:`Finished`
        (bind _ascar_bp (cast `/Game/CarModel/CarBP` _returnvalue))
        (set `/Game/CarModel/CarBP.Health` (`KismetMathLibrary.FMin` (+ (`/Game/CarModel/CarBP.Health` _ascar_bp) 25.0) 100.0) _ascar_bp)
        (`self.K2_DestroyActor`)))))

(fn `UserConstructionScript`)