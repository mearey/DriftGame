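; AI-driven boss car vehicle that takes throttle, brake and steering through events and whose death wins the game.
; Tick fires projectile volleys on a cooldown, turns the health bar toward the camera and rights the car when it rolls over.
; Projectile hits apply point damage and flash the mesh red, while debug keys damage the car.
; At zero health it spawns explosion effects in slow motion, destroys itself and opens the menu.
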(event `/Game/shooter_level/AI/BPI_isVehicle.SetThrottle`
  (params (Throttle :type "Float (double-precision)"))
  (`ChaosVehicleMovementComponent.SetThrottleInput` (`self.VehicleMovementComponent`) Throttle))

(event `/Game/shooter_level/AI/BPI_isVehicle.SetBrake`
  (params (Brake :type "Float (double-precision)"))
  (`ChaosVehicleMovementComponent.SetBrakeInput` (`self.VehicleMovementComponent`) Brake))

(event `/Game/shooter_level/AI/BPI_isVehicle.SetSteering`
  (params (Steering :type "Float (double-precision)"))
  (`ChaosVehicleMovementComponent.SetSteeringInput` (`self.VehicleMovementComponent`) Steering))

(event `self.ReceiveTick`
  (params (DeltaSeconds :type "Float (single-precision)"))
  (`self.ShootProjectiles`)
  (`self.UpdateHealthBar`)
  (`self.FlipIfNecessary`))

(event `ShootProjectiles`
  ;[1 1 1] projectiles
  (if (`self.CanAttack?`)
    (`|SpawnActorFromClass` "/Game/shooter_level/projectile/Projectile.Projectile_C" (`SceneComponent.K2_GetComponentToWorld` (`self.ProjectileLeftSpawnLocation`)) "Undefined" "MultiplyWithRoot" null null)
    (`|SpawnActorFromClass` "/Game/shooter_level/projectile/Projectile.Projectile_C" (`SceneComponent.K2_GetComponentToWorld` (`self.ProjectileForwardSpawnLocation`)) "Undefined" "MultiplyWithRoot" null null)
    (`|SpawnActorFromClass` "/Game/shooter_level/projectile/Projectile.Projectile_C" (`SceneComponent.K2_GetComponentToWorld` (`self.ProjectileRightSpawnLocation`)) "Undefined" "MultiplyWithRoot" null null)
    (`GameplayStatics.PlaySound2D` "/Game/shooter_level/projectile/ProjectileFireSound.ProjectileFireSound" 0.02 1.0 0.0 null null)
    (set `self.CanAttack?` false)
    (`KismetSystemLibrary.Delay` 0.5)
    (set `self.CanAttack?` true)))

(event `UpdateHealthBar`
  (bind _healthbarwidget (`self.HealthBarWidget`))
  ;[1 1 1] healthbar
  (bind _ashealth_bar (cast `/Game/shooter_level/HealthBar` (`WidgetComponent.GetWidget` (`self.HealthBarWidget`))))
  (`ProgressBar.SetPercent` (`/Game/shooter_level/HealthBar.ProgressBar` _ashealth_bar) (/ (`self.health`) 100.0))
  ;[1 1 1] healthbar rotation to camera
  (`SceneComponent.K2_SetWorldRotation` _healthbarwidget (`KismetMathLibrary.FindLookAtRotation` (`SceneComponent.K2_GetComponentLocation` _healthbarwidget) (`SceneComponent.K2_GetComponentLocation` (`PlayerCameraManager.TransformComponent` (`GameplayStatics.GetPlayerCameraManager` 0)))) false false))

(event `Key|Five`
  (params (Key :type "Key Structure"))
  (:`Pressed`
    (`KismetSystemLibrary.PrintString` "5 pressed")
    (`GameplayStatics.ApplyDamage` self 10.0)))

(event `self.ReceiveAnyDamage`
  (params (Damage :type "Float (single-precision)") (DamageType :type "DamageType Object Reference") (InstigatedBy :type "Controller Object Reference") (DamageCauser :type "Actor Object Reference"))
  ;[1 1 1] Damage
  (if (not (`self.isDead`))
    (bind _output_get (set `self.health` (- (`self.health`) Damage)))
    (if (<= _output_get 0.0)
      (`KismetSystemLibrary.PrintString` "Boss Died")
      (`self.AI_Kill`)
      (else
        (`KismetSystemLibrary.PrintString` (`KismetStringLibrary.Conv_DoubleToString` (`self.health`)))))))

(event `AI_Kill`
  (bind _returnvalue (`SceneComponent.K2_GetComponentLocation` (`self.Mesh`)))
  ;[1 1 1] BossKill
  (if (not (`self.isDead`))
    (set `self.isDead` true)
    (`GameplayStatics.SpawnEmitterAtLocation` "/Game/StarterContent/Particles/P_Fire.P_Fire" _returnvalue (struct) (5.0 5.0 5.0))
    (`GameplayStatics.SpawnEmitterAtLocation` "/Game/StarterContent/Particles/P_Explosion.P_Explosion" _returnvalue (struct) (20.0 20.0 20.0))
    (`GameplayStatics.SpawnSound2D` "/Game/StarterContent/Audio/Explosion01.Explosion01" 1.0 1.0 0.0 null)
    (`GameplayStatics.SetGlobalTimeDilation` 0.2)
    (`KismetSystemLibrary.Delay` 2.0)
    (`GameplayStatics.SetGlobalTimeDilation` 1.0)
    (`self.K2_DestroyActor`)
    (`self.PlayerWin`)))

(event `PlayerWin`
  ;[1 1 1] BossKill
  (`KismetSystemLibrary.PrintString` "GGs you won")
  (`GameplayStatics.OpenLevelBySoftObjectPtr` "/Game/menu/menu.menu"))

(event `Key|B`
  (params (Key :type "Key Structure"))
  (:`Pressed`
    (`GameplayStatics.ApplyDamage` self 10.0)))

(event `self.Mesh.OnComponentHit`
  (params (HitComponent :type "PrimitiveComponent Object Reference") (OtherActor :type "Actor Object Reference") (OtherComp :type "PrimitiveComponent Object Reference") (NormalImpulse :type "Vector Structure") (Hit :type "HitResult Structure (by ref)"))
  (bind (_bblockinghit _binitialoverlap _time _distance _location _impactpoint _normal _impactnormal _physmat _hitactor) (`GameplayStatics.BreakHitResult` Hit))
  (bind _asprojectile (cast `/Game/shooter_level/projectile/Projectile` OtherActor))
  (`GameplayStatics.ApplyPointDamage` _hitactor 10.0 _impactpoint Hit null _asprojectile)
  (`PrimitiveComponent.SetMaterial` (`self.Mesh`) 0 "/Game/shooter_level/Truck/M_Red.M_Red")
  (`KismetSystemLibrary.Delay` 0.5)
  (`PrimitiveComponent.SetMaterial` (`self.Mesh`) 0 "/Game/CarModel/Material_001.Material_001"))

(event `FlipIfNecessary`
  (bind _mesh (`self.Mesh`))
  (bind (_returnvalue_roll _returnvalue_pitch _returnvalue_yaw) (`KismetMathLibrary.BreakRotator` (`SceneComponent.K2_GetComponentRotation` _mesh)))
  (if (not (`KismetMathLibrary.InRange_FloatFloat` _returnvalue_roll -50.0 50.0))
    (`KismetSystemLibrary.PrintString` "must flip ai_carbp")
    (`self.K2_SetActorRotation` (`KismetMathLibrary.MakeRotator` 0.0) true)
    (`SceneComponent.K2_SetWorldRotation` _mesh (`KismetMathLibrary.MakeRotator` 0.0 _returnvalue_pitch _returnvalue_yaw) false true)))

(fn `DamageReset`
  (`PrimitiveComponent.SetMaterial` (`self.Mesh`) 0 "/Game/shooter_level/projectile/BaseMaterial.BaseMaterial"))

(fn `OnTakeDamage`
  (`PrimitiveComponent.SetMaterial` (`self.Mesh`) 0 "/Game/shooter_level/Truck/M_Red.M_Red"))

(fn `UserConstructionScript`)