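; AI-driven boss truck for the shooter level, whose death counts as the player's win.
; Exposes throttle, brake and steering events for an AI controller, while Tick fires cooldown-gated three-gun volleys, rights flipped trucks and turns the health bar to the camera.
; Player projectile hits apply damage with a red material flash, and low health starts a pulsing red overlay.
; Death triggers slow-motion explosions and impulses, shows player stats, then opens Level1.
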(event `self.ReceiveBeginPlay`
  ;[1 1 1] Event Begin Play
  (`SceneComponent.SetVisibility` (`self.HealthBarWidget`) false false)
  (`KismetSystemLibrary.Delay` 4.5)
  (`SceneComponent.SetVisibility` (`self.HealthBarWidget`) true false))

(event `/Game/shooter_level/AI/BPI_isVehicle.SetThrottle`
  (params (Throttle :type "Float (double-precision)"))
  ;[1 1 1] Using Ai Controller for following player
  (`ChaosVehicleMovementComponent.SetThrottleInput` (`self.VehicleMovementComponent`) Throttle))

(event `/Game/shooter_level/AI/BPI_isVehicle.SetBrake`
  (params (Brake :type "Float (double-precision)"))
  ;[1 1 1] Using Ai Controller for following player
  (`ChaosVehicleMovementComponent.SetBrakeInput` (`self.VehicleMovementComponent`) Brake))

(event `/Game/shooter_level/AI/BPI_isVehicle.SetSteering`
  (params (Steering :type "Float (double-precision)"))
  ;[1 1 1] Using Ai Controller for following player
  (`ChaosVehicleMovementComponent.SetSteeringInput` (`self.VehicleMovementComponent`) Steering))

(event `self.ReceiveTick`
  (params (DeltaSeconds :type "Float (single-precision)"))
  ;[1 1 1] Event Tick
  (`self.ShootProjectiles`)
  (`self.UpdateHealthWidget`)
  (`self.FlipIfNecessary`))

(event `ShootProjectiles`
  ;[0.9687 1 0.2204] projectiles
  (if (`self.CanAttack?`)
    (`|SpawnActorFromClass` "/Game/shooter_level/projectile/Projectile.Projectile_C" (`SceneComponent.K2_GetComponentToWorld` (`self.ProjectileLeftSpawnLocation`)) "Undefined" "MultiplyWithRoot" null null)
    (`|SpawnActorFromClass` "/Game/shooter_level/projectile/Projectile.Projectile_C" (`SceneComponent.K2_GetComponentToWorld` (`self.ProjectileForwardSpawnLocation`)) "Undefined" "MultiplyWithRoot" null null)
    (`|SpawnActorFromClass` "/Game/shooter_level/projectile/Projectile.Projectile_C" (`SceneComponent.K2_GetComponentToWorld` (`self.ProjectileRightSpawnLocation`)) "Undefined" "MultiplyWithRoot" null null)
    (`GameplayStatics.PlaySound2D` "/Game/shooter_level/projectile/ProjectileFireSound.ProjectileFireSound" 0.02 1.0 0.0 null null)
    (set `self.CanAttack?` false)
    (`KismetSystemLibrary.Delay` 2.0)
    (set `self.CanAttack?` true)))

(event `setIsLowHealth`
  ;[1 0.1765 0.1666] Draw red outline
  (bind (_direction _track_1) (`Timeline|Timeline` :!label _label)
    (:`Update`
      (if (> _track_1 0.5)
        (`MeshComponent.SetOverlayMaterial` (`self.Mesh`) "/Game/shooter_level/AI/M_OverlayRed.M_OverlayRed")
        (`MeshComponent.SetOverlayMaterial` (`self.GunForward`) "/Game/shooter_level/AI/M_OverlayRed.M_OverlayRed")
        (`MeshComponent.SetOverlayMaterial` (`self.GunLeft`) "/Game/shooter_level/AI/M_OverlayRed.M_OverlayRed")
        (`MeshComponent.SetOverlayMaterial` (`self.GunRight`) "/Game/shooter_level/AI/M_OverlayRed.M_OverlayRed")
        (else
          (`MeshComponent.SetOverlayMaterial` (`self.Mesh`) null)
          (`MeshComponent.SetOverlayMaterial` (`self.GunForward`) null)
          (`MeshComponent.SetOverlayMaterial` (`self.GunLeft`) null)
          (`MeshComponent.SetOverlayMaterial` (`self.GunRight`) null))))
    (:`Finished`
      (`KismetSystemLibrary.Delay` 0.2)
      (goto _label :!via `PlayFromStart`))))

(event `self.ReceiveAnyDamage`
  (params (Damage :type "Float (single-precision)") (DamageType :type "DamageType Object Reference") (InstigatedBy :type "Controller Object Reference") (DamageCauser :type "Actor Object Reference"))
  ;[1 1 1] Damage
  (`self.ApplyDamageToHealth` Damage))

(event `Boss_Kill`
  ;[1 0.5264 0.7361] BossKill
  (`self.IncrementPlayerBossKillCount`)
  (`self.ApplyBossDeathAnimation`)
  (`KismetSystemLibrary.Delay` 0.2)
  (`self.ShowPlayerStats`)
  (`RadialForceComponent.FireImpulse` (`self.RadialForce`))
  (`RadialForceComponent.FireImpulse` (`self.RadialForce1`))
  (`KismetSystemLibrary.Delay` 2.8)
  (`GameplayStatics.SetGlobalTimeDilation` 1.0)
  (`self.K2_DestroyActor`)
  (`self.PlayerWin`))

(event `PlayerWin`
  ;[1 0.5264 0.7361] BossKill
  (`KismetSystemLibrary.PrintString` "GGs you won")
  (`GameplayStatics.OpenLevelBySoftObjectPtr` "/Game/main_menu/Level1.Level1"))

(event `self.Mesh.OnComponentHit`
  (params (HitComponent :type "PrimitiveComponent Object Reference") (OtherActor :type "Actor Object Reference") (OtherComp :type "PrimitiveComponent Object Reference") (NormalImpulse :type "Vector Structure") (Hit :type "HitResult Structure (by ref)"))
  ;[1 1 1] On Truck Hit
  (`self.ApplyTruckDamage` OtherActor Hit)
  (`KismetSystemLibrary.Delay` 0.5)
  (`PrimitiveComponent.SetMaterial` (`self.Mesh`) 0 "/Game/shooter_level/AI/M_Enemy.M_Enemy"))

(event `FlipIfNecessary`
  (bind (_returnvalue_x _returnvalue_y _returnvalue_z) (`KismetMathLibrary.BreakVector` (`self.GetActorUpVector`)))
  (bind _returnvalue (`self.GetTransform`))
  (bind (_returnvalue_x_2 _returnvalue_y_2 _returnvalue_z_2) (`KismetMathLibrary.BreakVector` (`self.GetActorUpVector`)))
  ;[1 1 1] Flipping Truck if on side or upside down
  (if (`self.isDead`)
    _
    (elif (< _returnvalue_z_2 0.5)
      (`KismetSystemLibrary.Delay` 3.0)
      (if (< _returnvalue_z 0.2)
        (`self.K2_TeleportTo` (+ (.location _returnvalue) (0.0 0.0 200.0)) (`KismetMathLibrary.MakeRotator` 0.0 0.0 (.yaw (.rotation _returnvalue))))))))

(fn `ApplyBossDeathAnimation`
  (if (not (`self.isDead`))
    (set `self.isDead` true)
    (`SceneComponent.SetVisibility` (`self.HealthBarWidget`) false false)
    (`GameplayStatics.SpawnEmitterAttached` "/Game/StarterContent/Particles/P_Fire.P_Fire" (`self.Mesh`) "None" (0.0 0.0 0.0) (struct) (5.0 5.0 5.0))
    (`GameplayStatics.SpawnEmitterAttached` "/Game/shooter_level/explosiveBarrel/P_BarrelExplosion.P_BarrelExplosion" (`self.Mesh`))
    (`GameplayStatics.SpawnSound2D` "/Game/StarterContent/Audio/Explosion01.Explosion01" 1.0 1.0 0.0 null)
    (`GameplayStatics.SetGlobalTimeDilation` 0.2)))

(fn `ApplyDamageToHealth`
  (params (Damage :type "Float (double-precision)"))
  (`NiagaraFunctionLibrary.SpawnSystemAttached` "/Game/shooter_level/PowerUps/Effect_Damaged.Effect_Damaged" (`self.Mesh`) "None" (0.0 0.0 0.0) (struct) "KeepRelativeOffset")
  (if (not (`self.isDead`))
    (bind _output_get (set `self.health` (- (`self.health`) Damage)))
    (if (<= _output_get 0.0)
      (`KismetSystemLibrary.PrintString` "Boss Died")
      (`self.Boss_Kill`)
      (elif (<= _output_get 40.0)
        (`/Engine/EditorBlueprintResources/StandardMacros.DoOnce` false
          (:`Completed`
            (`self.setIsLowHealth`)))))))

(fn `ApplyTruckDamage`
  (params (OtherActor :type "Object Object Reference") (HitInfo :type "HitResult Structure (by ref)"))
  (bind (_bblockinghit _binitialoverlap _time _distance _location _impactpoint _normal _impactnormal _physmat _hitactor) (`GameplayStatics.BreakHitResult` HitInfo))
  (bind _asprojectile_special (cast `/Game/shooter_level/projectile/ProjectileSpecial` OtherActor)
    (:`then`
      (`GameplayStatics.ApplyPointDamage` _hitactor 50.0 _impactpoint HitInfo null _asprojectile_special))
    (:`CastFailed`
      (bind _asprojectile_player (cast `/Game/shooter_level/projectile/Projectile_Player` OtherActor))
      (`GameplayStatics.ApplyPointDamage` _hitactor 10.0 _impactpoint HitInfo null _asprojectile_player)))
  (`PrimitiveComponent.SetMaterial` (`self.Mesh`) 0 "/Game/shooter_level/Truck/M_Red.M_Red"))

(fn `DamageReset`
  (`PrimitiveComponent.SetMaterial` (`self.Mesh`) 0 "/Game/shooter_level/projectile/BaseMaterial.BaseMaterial"))

(fn `IncrementPlayerBossKillCount`
  (bind _ascar_bp_shooter (cast `/Game/shooter_level/CarBP_Shooter` (`GameplayStatics.GetPlayerPawn` 0)))
  (set `/Game/shooter_level/CarBP_Shooter.BossKilled` (+ (`/Game/shooter_level/CarBP_Shooter.BossKilled` _ascar_bp_shooter) 1) _ascar_bp_shooter)
  (set `/Game/shooter_level/CarBP_Shooter.HasWon` true _ascar_bp_shooter))

(fn `OnTakeDamage`
  (`PrimitiveComponent.SetMaterial` (`self.Mesh`) 0 "/Game/shooter_level/Truck/M_Red.M_Red"))

(fn `ShowPlayerStats`
  (bind _ascar_bp_shooter (cast `/Game/shooter_level/CarBP_Shooter` (`GameplayStatics.GetPlayerPawn` 0)))
  (`Widget.SetVisibility` (`/Game/shooter_level/CarBP_Shooter.PlayerStatsWidget` _ascar_bp_shooter) "Visible"))

(fn `UpdateHealthWidget`
  (bind _healthbarwidget (`self.HealthBarWidget`))
  ;[1 1 1] healthbar
  (bind _astruck_health_bar (cast `/Game/shooter_level/AI/TruckHealthBar` (`WidgetComponent.GetWidget` (`self.HealthBarWidget`))))
  (`ProgressBar.SetPercent` (`/Game/shooter_level/AI/TruckHealthBar.ProgressBar` _astruck_health_bar) (/ (`self.health`) 100.0))
  ;[1 1 1] healthbar rotation to camera
  (`SceneComponent.K2_SetWorldRotation` _healthbarwidget (`KismetMathLibrary.FindLookAtRotation` (`SceneComponent.K2_GetComponentLocation` _healthbarwidget) (`SceneComponent.K2_GetComponentLocation` (`PlayerCameraManager.TransformComponent` (`GameplayStatics.GetPlayerCameraManager` 0)))) false false))

(fn `UserConstructionScript`)